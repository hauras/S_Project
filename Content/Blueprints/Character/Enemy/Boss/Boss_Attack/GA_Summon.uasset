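; GA_Summon is a boss Gameplay Ability that summons an enemy around the boss.
; A SpawnEnemies task, given the Event.Montage.Summon tag, is set to spawn one configured enemy class within a random radius, using the boss's forward rotation.
; The summon montage starts right after the task, and any montage outcome clears a boolean Blackboard key on the AI controller and ends the ability.
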(event `self.K2_ActivateAbility`
  (`AbilityTask_SpawnEnemy.SpawnEnemies` self (struct :`TagName` "Event.Montage.Summon") (`self.Enemy Class to Spawn`) 1 (`Actor.K2_GetActorLocation` (`self.GetAvatarActorFromActorInfo`)) 600.0 (`KismetMathLibrary.Conv_VectorToRotator` (`Actor.GetActorForwardVector` (`self.GetAvatarActorFromActorInfo`)))
    (:`then`
      (`AbilityTask_PlayMontageAndWait.CreatePlayMontageAndWaitProxy` "None" (`self.Montage to Play`)
        (:`OnCompleted`
          _)
        (:`OnBlendOut`
          _)
        (:`OnInterrupted`
          _)
        (:`OnCancelled`
          _))
      (`BlackboardComponent.SetValueAsBool` (`AIBlueprintHelperLibrary.GetBlackboard` (`AIBlueprintHelperLibrary.GetAIController` (`self.GetAvatarActorFromActorInfo`))) (`self.Key Name`) false)
      (`self.K2_EndAbility`))))